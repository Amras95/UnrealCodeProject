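; BP_Door_2 is a door Blueprint that opens by moving its static mesh vertically.
; BeginPlay caches the mesh's world location, and OpenDoor plays the ElevatePlatform timeline, adding its ZAxis track to that location as a height offset.
; CloseDoor is an empty event, and the rotation-based closing nodes are left unconnected, so the graph has no working close behaviour.
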(event `self.ReceiveBeginPlay`
  (set `self.DefaultLocation` (`SceneComponent.K2_GetComponentLocation` (`self.StaticMesh`))))

(event `OpenDoor`
  ;[1 1 1] DoorRotation
  (bind (_direction _zaxis) (`Timeline|ElevatePlatform`)
    (:`Update`
      (`SceneComponent.K2_SetWorldLocation` (`self.StaticMesh`) (+ (`KismetMathLibrary.MakeVector` 0.0 0.0 _zaxis) (`self.DefaultLocation`)) false false))))

(event `CloseDoor`
  ;[1 1 1] Close Door
)

(fn `UserConstructionScript`)