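; BP_Puzzle is an interactable three-key rotation puzzle that opens a door when the keys match a code.
; Interact yaws the passed component by a fixed step, though left rotation always turns FirstKey, and prints the component's rotation.
; CheckCode compares that component's yaw to its Code entry within a tolerance and stores the result in CorrectCode.
; The Door opens when every entry is correct and closes otherwise.
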(event `/Game/Interfaces/BP_GameplayInterface.Interact`
  (params (CharacterPawn :type "PrimitiveComponent Object Reference") (RotateLeft :type Boolean))
  (`self.Rotate` RotateLeft CharacterPawn))

(fn `CheckCode`
  (params (Component :type "PrimitiveComponent Object Reference"))
  (locals (SelectedMesh :type Integer) (LocalFailed :type Boolean))
  (bind _door (`self.Door`))
  (bind (_relativerotation_roll _relativerotation_pitch _relativerotation_yaw) (`KismetMathLibrary.BreakRotator` (`SceneComponent.RelativeRotation` Component)))
  (if (== Component (`self.FirstKey`))
    (set `local.SelectedMesh` 0)
    (`KismetArrayLibrary.Array_Set` (`self.CorrectCode`) (`local.SelectedMesh`) (`KismetMathLibrary.NearlyEqual_FloatFloat` (`|GetArrayItem` (`self.Code`) (`local.SelectedMesh`)) _relativerotation_yaw 35.0) :!label _label)
    (for _array_element (`self.CorrectCode`)
      (if (not _array_element)
        (set `local.LocalFailed` true)))
    (if (`local.LocalFailed`)
      (`/Game/GameplayContent/BP_Door_2.CloseDoor` _door)
      (else
        (`/Game/GameplayContent/BP_Door_2.OpenDoor` _door)))
    (elif (== Component (`self.SecondKey`))
      (set `local.SelectedMesh` 1)
      (goto _label)
      (elif (== Component (`self.ThirdKey`))
        (set `local.SelectedMesh` 2)
        (goto _label)))))

(fn `Rotate`
  (params (RotateLeft :type Boolean) (Component :type "PrimitiveComponent Object Reference"))
  (if RotateLeft
    (`SceneComponent.K2_AddRelativeRotation` (`self.FirstKey`) (`KismetMathLibrary.MakeRotator` 0.0 0.0 (* (`self.RotationValue`) -1.0)) false false)
    (else
      (`SceneComponent.K2_AddRelativeRotation` Component (`KismetMathLibrary.MakeRotator` 0.0 0.0 (`self.RotationValue`)) false false)))
  (`KismetSystemLibrary.PrintString` (`KismetStringLibrary.Conv_RotatorToString` (`SceneComponent.RelativeRotation` Component)))
  (`self.CheckCode` Component))

(fn `UserConstructionScript`)